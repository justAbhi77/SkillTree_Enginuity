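; Skill tree vendor Blueprint that opens a vendor UI through a proximity trigger sphere.
; On begin overlap it lazily creates and caches the vendor widget, adds it to the viewport, switches to game-and-UI input and shows the cursor.
; End overlap removes the widget and restores game-only input with a hidden cursor.
; Neither event checks which actor overlaps, and both target player controller 0.
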(event `self.Sphere.OnComponentBeginOverlap`
  (params (OverlappedComponent :type "PrimitiveComponent Object Reference") (OtherActor :type "Actor Object Reference") (OtherComp :type "PrimitiveComponent Object Reference") (OtherBodyIndex :type Integer) (bFromSweep :type Boolean) (SweepResult :type "HitResult Structure (by ref)"))
  (bind _returnvalue (`GameplayStatics.GetPlayerController` 0))
  (`|ExecutionSequence`
    (:`then_0`
      (`self.VendorWidget`
        (:`then`)
        (:`else`
          (bind _returnvalue_2 (`|CreateWidget` "/Game/SkillTree/Vendor/Wbp_SkillTree_Vendor.Wbp_SkillTree_Vendor_C"))
          (set `self.VendorWidget` _returnvalue_2))))
    (:`then_1`
      (`UserWidget.AddToViewport` (`self.VendorWidget`) 0)
      (`WidgetBlueprintLibrary.SetInputMode_GameAndUIEx` _returnvalue (`self.VendorWidget`))
      (set `PlayerController.bShowMouseCursor` true _returnvalue))))

(event `self.Sphere.OnComponentEndOverlap`
  (params (OverlappedComponent :type "PrimitiveComponent Object Reference") (OtherActor :type "Actor Object Reference") (OtherComp :type "PrimitiveComponent Object Reference") (OtherBodyIndex :type Integer))
  (bind _returnvalue (`GameplayStatics.GetPlayerController` 0))
  (bind _vendorwidget (`self.VendorWidget`)
    (:`then`
      (`Widget.RemoveFromParent` _vendorwidget)
      (`WidgetBlueprintLibrary.SetInputMode_GameOnly` _returnvalue)
      (set `PlayerController.bShowMouseCursor` false _returnvalue))
    (:`else`)))

(fn `UserConstructionScript`)