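; Player controller component that opens and closes the skill tree UI and supplies its node data and layout settings.
; On non-server instances it remaps configurable keys to the toggle input action at BeginPlay, then sends an initial toggle.
; Opening async-loads the soft widget class, fades it in and enables cursor input; closing fades it out and restores game-only input.
; Getters return the node DataTable and tree display settings, rescaling blur and brightness and offsetting rotation.
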(event `self.ReceiveBeginPlay`
  (if (not (`KismetSystemLibrary.IsDedicatedServer`))
    (`EnhancedInputSubsystemInterface.AddMappingContext` (pcsubsystem `EnhancedInputLocalPlayerSubsystem` (`GameplayStatics.GetPlayerController` 0)) (`self.Mapping Context`) 0 (struct))
    (`InputMappingContext.UnmapAll` (`self.Mapping Context`))
    (for _array_element (`self.OpenCloseWidgetKeys`)
      (`InputMappingContext.MapKey` (`self.Mapping Context`) "/Game/SkillTree/MiscData/Input/Ia_SkillTree.Ia_SkillTree" _array_element))
    (message `/Game/SkillTree/MiscData/Interfaces/Bpi_SkillTree_PlayerContComp.eOpenCloseSkillTree` (`/Game/SkillTree/MiscData/FunctionLibraries/Bfl_SkillTree.BflGetSkillTreeComp`))))

(event `EnhancedInput|/Game/SkillTree/MiscData/Input/Ia_SkillTree`
  (params (ActionValue :type Boolean) (ElapsedSeconds :type "Float (double-precision)") (TriggeredSeconds :type "Float (double-precision)") (InputAction :type "InputAction Object Reference" :default "/Game/SkillTree/MiscData/Input/Ia_SkillTree.Ia_SkillTree"))
  (:`Triggered`
    (message `/Game/SkillTree/MiscData/Interfaces/Bpi_SkillTree_PlayerContComp.eOpenCloseSkillTree` (`/Game/SkillTree/MiscData/FunctionLibraries/Bfl_SkillTree.BflGetSkillTreeComp`))))

(event `/Game/SkillTree/MiscData/Interfaces/Bpi_SkillTree_PlayerContComp.eOpenCloseSkillTree`
  (bind _returnvalue (`GameplayStatics.GetPlayerController` 0))
  (if (not (`KismetSystemLibrary.IsDedicatedServer`))
    (bind _skilltreewidget (`self.SkillTreeWidget`)
      (:`then`
        (message `/Game/SkillTree/MiscData/Interfaces/Bpi_SkillTree_BaseWidget.eFadeOutThenDestroy` _skilltreewidget)
        (set `self.SkillTreeWidget` null)
        (`WidgetBlueprintLibrary.SetInputMode_GameOnly` _returnvalue)
        (set `PlayerController.bShowMouseCursor` false _returnvalue))
      (:`else`
        (`self.eCreateUi`)))))

(event `eCreateUi`
  (bind _returnvalue (`GameplayStatics.GetPlayerController` 0))
  (bind _class (`|LoadAssetClass` (`self.SkillTreeWidgetSoftClass`))
    (:`Completed`
      (bind _asuser_widget (castclass `UserWidget` _class))
      (bind _returnvalue_2 (`|CreateWidget` _asuser_widget (`GameplayStatics.GetPlayerController` 0)))
      (bind _output_get (set `self.SkillTreeWidget` _returnvalue_2))
      (`UserWidget.AddToViewport` _output_get 0)
      (`WidgetBlueprintLibrary.SetInputMode_GameAndUIEx` _returnvalue (`self.SkillTreeWidget`) "LockAlways" false)
      (set `PlayerController.bShowMouseCursor` true _returnvalue)
      (message `/Game/SkillTree/MiscData/Interfaces/Bpi_SkillTree_BaseWidget.eFadeIn` (`self.SkillTreeWidget`)))))

(fn `fGetNodeInfo`
  (returns (DataTable :type "DataTable Object Reference"))
  (return (`self.Data Table`)))

(fn `fGetTreeInfo`
  (returns (PanningSpeed :type "Float (double-precision)") (StartingZoom :type "Float (double-precision)") (ZoomInClamp :type "Float (double-precision)") (ZoomOutClamp :type "Float (double-precision)") (ZoomDuration :type "Float (double-precision)") (BackgroundBlur :type "Float (double-precision)") (BackgroundBrightness :type "Float (double-precision)") (StartingOffset :type "Vector2D Structure") (bFlipMouseWheel :type Boolean) (TreeRotation :type "Float (double-precision)") (DegreeSpan :type "Float (double-precision)") (TierDistance :type "Float (double-precision)") (EdgeBuffer :type "Float (double-precision)") (bCounterClockwise :type Boolean) (ConnectorWidth :type "Float (double-precision)") (ConnectorEndTrimming :type "Float (double-precision)"))
  (return (`self.Panning Speed`) (`self.Starting Zoom`) (`self.Zoom in Clamp`) (`self.Zoom Out Clamp`) (`self.Zoom Duration`) (* (`self.Background Blur`) 200.0) (* (`self.Background Brightness`) 3.0) (`self.Starting Offset`) (`self.bFlipMouseWheel`) (- (`self.TreeRotation`) 90.0) (`self.DegreeSpan`) (`self.TierDistance`) (`self.EdgeBuffer`) (`self.bCounterClockwise`) (`self.Connector Width`) (`self.Connector End Trimming`)))